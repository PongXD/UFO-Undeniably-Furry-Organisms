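; BP_Switch is a replicated puzzle pressure button that opens or closes linked gates when matching pawns enter or leave its radius.
; Overlapping pawns qualify by required shape or material, and the button releases when no valid pawn remains.
; Toggling runs a press timeline and calls ActivateDoor on each gate, while RepNotifies handle click sounds and number transparency.
; Dynamic materials display the requirement beneath a spinning, hovering index number.
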(event OnComponentBeginOverlap(CollisionRadius)
  (params (OverlappedComponent :type Primitive%20Component%20Object%20Reference) (OtherActor :type Actor%20Object%20Reference) (OtherComp :type Primitive%20Component%20Object%20Reference) (OtherBodyIndex :type Integer) (bFromSweep :type Boolean) (SweepResult :type Hit%20Result%20Structure%20%28by%20ref%29))
  ;[1 1 1] Overlap events with pawns
  (bind _isvalid (CallFunction|CheckValid OtherActor))
  (if _isvalid
    (Utilities|Array|AddUnique (Variables|Default|GetPawnsActivatingThis) OtherActor)
    (if (not (Variables|Default|GetisPushedDown))
      (CallFunction|ActivateButton))))

(event OnComponentEndOverlap(CollisionRadius)
  (params (OverlappedComponent :type Primitive%20Component%20Object%20Reference) (OtherActor :type Actor%20Object%20Reference) (OtherComp :type Primitive%20Component%20Object%20Reference) (OtherBodyIndex :type Integer))
  (bind _pawnsactivatingthis (Variables|Default|GetPawnsActivatingThis))
  ;[1 1 1] Overlap events with pawns
  (Variables|Default|SetButtonChange true)
  (Utilities|Array|RemoveItem _pawnsactivatingthis OtherActor)
  (bind _array_element (Utilities|Array|ForEachLoopwithBreak _pawnsactivatingthis :!label _label)
    (:LoopBody
      (bind _isvalid (CallFunction|CheckValid _array_element))
      (if _isvalid
        (Variables|Default|SetButtonChange false)
        (goto _label Break)))
    (:Completed
      (if (and (Variables|Default|GetButtonChange) (Variables|Default|GetisPushedDown))
        (CallFunction|ActivateButton)))))

(event Custom|ActivateButton
  ;[1 1 1] Activate switch
  (Utilities|FlowControl|Sequence
    (:then_0
      (CallFunction|ButtonAnimation (Variables|Default|GetisPushedDown)))
    (:then_1
      (bind _output_get (Variables|Default|SetisPushedDown (not (Variables|Default|GetisPushedDown))))
      (for _array_element (Variables|Default|GetGatesToActivate)
        (Default|ActivateDoor _array_element _output_get)))))

(event Custom|ButtonAnimation
  (params (isButtonDown :type Boolean))
  ;[1 1 1] Button Animation
  (if isButtonDown
    (bind (_direction _buttondownvalue _transparencyvalue) (Timeline|ButtonTimeline Reverse)
      (:Update
        (Transformation|SetRelativeLocation (Variables|Default|GetButton) (Math|Vector|MakeVector 0.0 0.0 (* _buttondownvalue 1e+01)) false false)
        (Variables|Default|SetNumberTransparency _transparencyvalue)))
    (else
      (Timeline|ButtonTimeline Play))))

(event Custom|PrintArray
  (for _array_element (Variables|Default|GetPawnsActivatingThis)
    (Development|PrintString (Utilities|GetDisplayName _array_element))))

(event EventBeginPlay
  (bind _dmi_buttonmat (Variables|Default|GetDMI_ButtonMat))
  (bind _dmi_buttonmat_2 (Variables|Default|GetDMI_ButtonMat))
  ;[1 1 1] Setting the details of the switch
  (Rendering|Components|TextRender|SetText (Variables|Default|GetSwitchNumber) (Utilities|Text|ToText(Integer) (Variables|Default|GetSwitchIndex)))
  (Utilities|FlowControl|Sequence
    (:then_0
      (switch int (Variables|Default|GetRequiredShapeIndex)
        (:0
          (Rendering|Material|SetTextureParameterValue _dmi_buttonmat "Picture" "/Game/Levels/PuzzleLevels/Pictures/white_square_corner.white_square_corner"))
        (:1
          (Rendering|Material|SetTextureParameterValue _dmi_buttonmat "Picture" "/Game/Levels/PuzzleLevels/Pictures/white_circle_corner.white_circle_corner"))
        (:2
          (Rendering|Material|SetTextureParameterValue _dmi_buttonmat "Picture" "/Game/Levels/PuzzleLevels/Pictures/white_triangle_corner.white_triangle_corner"))))
    (:then_1
      (switch int (Variables|Default|GetRequiredMaterialIndex)
        (:0
          (Rendering|Material|SetVectorParameterValue _dmi_buttonmat_2 "Color" "(R=0.049769,G=0.288011,B=0.800000,A=1.000000)" :!class /Script/Engine.MaterialInstanceDynamic))
        (:1
          (Rendering|Material|SetVectorParameterValue _dmi_buttonmat_2 "Color" "(R=0.400000,G=0.400000,B=0.400000,A=1.000000)" :!class /Script/Engine.MaterialInstanceDynamic))))))

(event EventTick
  (params (DeltaSeconds :type Float%20%28single-precision%29))
  (bind _switchnumber (Variables|Default|GetSwitchNumber))
  ;[1 1 1] Rotation of number
  (bind (_direction _rotationvalue _hovervalue) (Timeline|Rotation Play)
    (:Update
      (Transformation|SetRelativeRotation _switchnumber (Math|Rotator|MakeRotator 0.0 0.0 (* _rotationvalue 7.2e+02)) false false)
      (Transformation|SetRelativeLocation _switchnumber (Math|Vector|MakeVector 0.0 0.0 (+ (* _hovervalue 1e+01) 4e+01)) false false))))

(fn ConstructionScript
  (bind _returnvalue (Rendering|Material|CreateDynamicMaterialInstance (Variables|Default|GetSwitchNumber) 0 0 :!class /Script/Engine.PrimitiveComponent))
  (Variables|Default|SetDMI_Transparency _returnvalue)
  (bind _returnvalue_2 (Rendering|Material|CreateDynamicMaterialInstance (Variables|Default|GetButton) 0 0 :!class /Script/Engine.PrimitiveComponent))
  (Variables|Default|SetDMI_ButtonMat _returnvalue_2)
  (Class|ActorComponent|SetIsReplicated (Variables|Default|GetButton) true)
  (Class|ActorComponent|SetIsReplicated (Variables|Default|GetSwitchNumber) true))

(fn CheckValid
  (params (ActorOnButton :type Actor%20Object%20Reference))
  (bind _ispossessed (Class|BPIInteract|IsPossessed(Message) ActorOnButton))
  (if _ispossessed
    (bind (_shape _phymaterial) (Class|BPIInteract|GetDetails(Message) ActorOnButton)))
  (return (or (and (== _shape (Variables|Default|GetRequiredShapeIndex)) (!= _shape -1)) (and (== _phymaterial (Variables|Default|GetRequiredMaterialIndex)) (!= _phymaterial -1)))))

(fn OnRepNumberTransparency
  (Rendering|Material|SetScalarParameterValue (Variables|Default|GetDMI_Transparency) "Transparency" (Variables|Default|GetNumberTransparency) :!class /Script/Engine.MaterialInstanceDynamic))

(fn OnRepIsPushedDown
  (bind _returnvalue (Transformation|GetActorLocation))
  (if (Variables|Default|GetisPushedDown)
    (Audio|SpawnSoundatLocation "/Game/Levels/PuzzleLevels/Audio/Button_Click_On.Button_Click_On" _returnvalue)
    (else
      (Audio|SpawnSoundatLocation "/Game/Levels/PuzzleLevels/Audio/Button_Click_Off.Button_Click_Off" _returnvalue))))