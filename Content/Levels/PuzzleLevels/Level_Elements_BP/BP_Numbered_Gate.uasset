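; Numbered puzzle gate that displays its GateIndex and slides vertically between closed and raised positions, with StartingStatus letting it begin raised.
; ActivateDoor compares the button state to StartingStatus, so a starting-open gate responds inversely, then plays or reverses the UpDown timeline that offsets the gate from its original location.
; It also sets DoorOpenCloseIndex, whose RepNotify plays the elevator door open or close sound at the gate.
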(event Custom|ActivateDoor
  (params (isButtonPushed :type Boolean))
  (if (Math|Boolean|NotEqual(Boolean) isButtonPushed (Variables|Default|GetStartingStatus))
    (Variables|Default|SetDoorOpenCloseIndex 0)
    (bind _value (Timeline|Up&Down Play)
      (:Update
        (Transformation|SetActorLocation (+ (* "0, 0,350.000000" _value) (Variables|Default|GetOGLocation)) false false)))
    (else
      (Variables|Default|SetDoorOpenCloseIndex 1)
      (Timeline|Up&Down Reverse))))

(event Collision|EventActorBeginOverlap
  (params (OtherActor :type Actor%20Object%20Reference)))

(event EventTick
  (params (DeltaSeconds :type Float%20%28single-precision%29)))

(event EventBeginPlay
  (Variables|Default|SetOGLocation (Transformation|GetActorLocation))
  (if (Variables|Default|GetStartingStatus)
    (Utilities|FlowControl|Sequence
      (:then_0
        (Transformation|AddActorLocalOffset "0, 0,350.000000" false false)
        (Rendering|Components|TextRender|SetText (Variables|Default|GetDoorNumber) (Utilities|Text|ToText(Integer) (Variables|Default|GetGateIndex)) :!label _label))
      (:then_1
        (bind _value (Timeline|Up&Down SetNewTime)
          (:Update
            (Transformation|SetActorLocation (+ (* "0, 0,350.000000" _value) (Variables|Default|GetOGLocation)) false false)))))
    (else
      (goto _label))))

(fn ConstructionScript)

(fn OnRepDoorOpenCloseIndex
  (bind _returnvalue (Transformation|GetActorLocation))
  (switch int (Variables|Default|GetDoorOpenCloseIndex)
    (:0
      (Audio|SpawnSoundatLocation "/Game/Levels/PuzzleLevels/Audio/elevator_door_open_Cue.elevator_door_open_Cue" _returnvalue))
    (:1
      (Audio|SpawnSoundatLocation "/Game/Levels/PuzzleLevels/Audio/elevator_door_close_Cue.elevator_door_close_Cue" _returnvalue))))