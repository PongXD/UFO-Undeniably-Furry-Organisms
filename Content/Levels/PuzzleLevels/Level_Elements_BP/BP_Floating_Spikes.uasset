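; Floating spike hazard for puzzle levels that kills and respawns actors touching its collision area, unless they are made of metal.
; On overlap it reads the other actor's physical material through a details message, then for non-metal plays a sound at that actor, sends it a death-and-respawn message and prints debug text.
; The construction script gives both blocking volume components dynamic materials showing the spikes texture.
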(event OnComponentBeginOverlap(CollisionArea)
  (params (OverlappedComponent :type Primitive%20Component%20Object%20Reference) (OtherActor :type Actor%20Object%20Reference) (OtherComp :type Primitive%20Component%20Object%20Reference) (OtherBodyIndex :type Integer) (bFromSweep :type Boolean) (SweepResult :type Hit%20Result%20Structure%20%28by%20ref%29))
  (bind _phymaterial (Class|BPIInteract|GetDetails(Message) OtherActor))
  (if (not (== _phymaterial 1))
    (Audio|SpawnSoundatLocation "/Game/Levels/PuzzleLevels/Audio/Blop-Mark_DiAngelo_Cue.Blop-Mark_DiAngelo_Cue" (Transformation|GetActorLocation OtherActor))
    (Class|BPIInteract|DeathandRespawn(Message) OtherActor)
    (Development|PrintString "DEATH by PENETRATION!!!")))

(fn ConstructionScript
  (bind _returnvalue (Rendering|Material|CreateDynamicMaterialInstance (Variables|Default|GetBlockingVolume) 0 0 :!class /Script/Engine.PrimitiveComponent))
  (bind _output_get (Variables|Default|SetDMI_Picture _returnvalue))
  (Rendering|Material|SetTextureParameterValue _output_get "Picture" "/Game/Levels/PuzzleLevels/Pictures/spikes.spikes")
  (bind _returnvalue_2 (Rendering|Material|CreateDynamicMaterialInstance (Variables|Default|GetBlockingVolume2) 0 0 :!class /Script/Engine.PrimitiveComponent))
  (bind _output_get_2 (Variables|Default|SetDMI_Picture_Btm _returnvalue_2))
  (Rendering|Material|SetTextureParameterValue _output_get_2 "Picture" "/Game/Levels/PuzzleLevels/Pictures/spikes.spikes"))