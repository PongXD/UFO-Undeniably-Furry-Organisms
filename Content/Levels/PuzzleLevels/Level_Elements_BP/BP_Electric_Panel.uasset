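; Electrified floor panel hazard for puzzle levels that kills and respawns overlapping actors unless they are made of rubber.
; On collision overlap it reads the actor's physical material through a details message; any non-rubber type triggers an energy burst sound, a death-and-respawn message and a debug print.
; The construction script gives the panel a dynamic material instance showing a lightning symbol.
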(event OnComponentBeginOverlap(CollisionArea)
  (params (OverlappedComponent :type Primitive%20Component%20Object%20Reference) (OtherActor :type Actor%20Object%20Reference) (OtherComp :type Primitive%20Component%20Object%20Reference) (OtherBodyIndex :type Integer) (bFromSweep :type Boolean) (SweepResult :type Hit%20Result%20Structure%20%28by%20ref%29))
  (bind _phymaterial (Class|BPIInteract|GetDetails(Message) OtherActor))
  (if (not (== _phymaterial 0))
    (Audio|PlaySoundatLocation "/Game/Levels/PuzzleLevels/Audio/magical_energy_burst_1sec_Cue.magical_energy_burst_1sec_Cue" (Transformation|GetActorLocation OtherActor))
    (Class|BPIInteract|DeathandRespawn(Message) OtherActor)
    (Development|PrintString "DEATH by ELECTROCUTION!!")))

(fn ConstructionScript
  (bind _returnvalue (Rendering|Material|CreateDynamicMaterialInstance (Variables|Default|GetFloorPanel) 0 0 :!class /Script/Engine.PrimitiveComponent))
  (bind _output_get (Variables|Default|SetDMI_Picture _returnvalue))
  (Rendering|Material|SetTextureParameterValue _output_get "Picture" "/Game/Levels/PuzzleLevels/Pictures/Lightning_symbol.Lightning_symbol"))